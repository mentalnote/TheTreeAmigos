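; Building Blueprint that defines placement rules and Sunlight and Water costs for constructing on a tile.
; CanConstruct requires the tile's ground building class to match RequiredBase exactly, or an empty tile when no base is required.
; It then checks both costs against the Currency held by MainGameMode, without spending it.
; The construction script only prints the RequiredBase class default SunlightCost, apparently as debug output.
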(fn `CanConstruct`
  (params (Tile :type "/Game/Blueprints/Tile Object Reference"))
  (returns (CanConstruct :type Boolean))
  (bind _groundbuilding (`/Game/Blueprints/Tile.GroundBuilding` Tile))
  (`/Engine/EditorBlueprintResources/StandardMacros.IsValid` _groundbuilding
    (:`Is Valid`
      (if (== (`GameplayStatics.GetObjectClass` _groundbuilding) (`self.RequiredBase`))
        (bind _asmain_game_mode (cast `/Game/Blueprints/MainGameMode` (`GameplayStatics.GetGameMode`) :!label _label)
          (:`then`
            (bind _currency (`/Game/Blueprints/MainGameMode.Currency` _asmain_game_mode))
            (bind _sunlight (`/Game/Blueprints/Currency.GetSunlight` _currency))
            (if (<= (`self.SunlightCost`) _sunlight)
              (bind _water (`/Game/Blueprints/Currency.GetWater` _currency))
              (if (<= (`self.WaterCost`) _water)
                (return true)
                (else
                  _))))
          (:`CastFailed`
            _))))
    (:`Is Not Valid`
      (if (!= (`self.RequiredBase`) null)
        _
        (else
          (goto _label)))))
  (return false))

(fn `UserConstructionScript`
  (`KismetSystemLibrary.PrintString` (`KismetStringLibrary.Conv_IntToString` (defaults `/Game/Blueprints/Buildings/Building` (`self.RequiredBase`)))))