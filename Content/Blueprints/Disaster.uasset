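; Disaster actor that steps tile by tile toward the main tree each end turn, showing the lose widget if it lands there.
; It picks the neighbour by 60-degree yaw toward the tree, affects the entered tile and spawns an indicator on the next.
; Brambles or UmbrellaLeaf on the tile destroy matching ground or air disasters.
; Tick drains a movement queue as one-second arcing hops, separating visuals from tile logic.
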(event `self.ReceiveBeginPlay`
  (bind _asmain_game_mode (cast `/Game/Blueprints/MainGameMode` (`GameplayStatics.GetGameMode`)))
  (add `/Game/Blueprints/MainGameMode.EndTurn` _asmain_game_mode (delegate `ProcessTurn`)))

(event `ProcessTurn`
  (bind _item (`self.GetNextMovementTile`))
  (`/Engine/EditorBlueprintResources/StandardMacros.IsValid` _item
    (:`Is Valid`
      (`self.MoveToTile` _item)
      (`/Game/Blueprints/Tile.AffectTile` (`self.Tile`) self)
      (`self.K2_DestroyActor` (`self.MovementIndicator`))
      (bind _item_2 (`self.GetNextMovementTile`))
      (bind _returnvalue (`|SpawnActorFromClass` (`self.MovementIndicatorClass`) (`self.GetTransform` _item_2) "AlwaysSpawn" "OverrideRootScale"))
      (bind _output_get (set `self.MovementIndicator` _returnvalue))
      (`self.SetActorScale3D` _output_get (5.0 5.0 5.0)))))

(event `self.ReceiveTick`
  (params (DeltaSeconds :type "Float (single-precision)"))
  (bind _movementqueue (`self.MovementQueue`))
  (bind _item (`KismetArrayLibrary.Array_Get` (`self.MovementQueue`)))
  (bind _returnvalue (/ (`self.MovementQueueTime`) 1.0))
  (if (> (`KismetArrayLibrary.Array_Length` (`self.MovementQueue`)) 1)
    (set `self.MovementQueueTime` (- (`self.MovementQueueTime`) DeltaSeconds))
    (if (> (`self.MovementQueueTime`) 0.0)
      (`self.K2_SetActorLocation` (+ (`KismetMathLibrary.VLerp` (`self.K2_GetActorLocation` _item) (`self.K2_GetActorLocation` (`KismetArrayLibrary.Array_Get` _movementqueue 1)) (- 1.0 _returnvalue)) (`KismetMathLibrary.VLerp` (0.0 0.0 0.0) (0.0 0.0 200.0) (- 1.0 (`KismetMathLibrary.Abs` (* (- _returnvalue 0.5) 2.0))))) false true)
      (else
        (`KismetArrayLibrary.Array_Remove` _movementqueue)
        (set `self.MovementQueueTime` (+ (`self.MovementQueueTime`) 1.0))))
    (else
      (`self.K2_SetActorLocation` (`self.K2_GetActorLocation` _item) false true)
      (set `self.MovementQueueTime` 1.0))))

(fn `GetNextMovementTile`
  (returns (Item :type "/Game/Blueprints/Tile Object Reference"))
  (bind _asmain_game_mode (cast `/Game/Blueprints/MainGameMode` (`GameplayStatics.GetGameMode`))
    (:`then`
      (bind _yaw (.yaw (`KismetMathLibrary.Conv_VectorToRotator` (- (`self.K2_GetActorLocation` (`KismetArrayLibrary.Array_Get` (`/Game/Blueprints/MainGameMode.MainTreeTiles` _asmain_game_mode))) (`self.K2_GetActorLocation` (`self.Tile`))))))
      (return (`KismetArrayLibrary.Array_Get` (`/Game/Blueprints/Tile.Neighbours` (`self.Tile`)) (`KismetMathLibrary.FTrunc` (+ (/ (`KismetMathLibrary.SelectFloat` (+ 360.0 _yaw) _yaw (< _yaw 0.0)) 60.0) 0.5)))))
    (:`CastFailed`
      (return null))))

(fn `MoveToTile`
  (params (NewTile :type "/Game/Blueprints/Tile Object Reference") (Force :type Boolean))
  (bind _tile (`self.Tile`))
  (`/Engine/EditorBlueprintResources/StandardMacros.IsValid` NewTile
    (:`Is Valid`
      (`/Engine/EditorBlueprintResources/StandardMacros.IsValid` (`self.Tile`)
        (:`Is Valid`
          (set `/Game/Blueprints/Tile.Disaster` null (`self.Tile`)))
        (:`Is Not Valid`
          _))
      (if (or Force (not (`KismetSystemLibrary.IsValid` (`/Game/Blueprints/Tile.Disaster` NewTile))))
        (bind _output_get (set `self.Tile` NewTile))
        (bind _disaster (`/Game/Blueprints/Tile.Disaster` _output_get))
        (`/Engine/EditorBlueprintResources/StandardMacros.IsValid` _disaster
          (:`Is Valid`
            (set `/Game/Blueprints/Disaster.Tile` null _disaster))
          (:`Is Not Valid`
            _))
        (set `/Game/Blueprints/Tile.Disaster` self _output_get)
        (`KismetArrayLibrary.Array_Add` (`self.MovementQueue`) _output_get)
        (bind _asmain_game_mode (cast `/Game/Blueprints/MainGameMode` (`GameplayStatics.GetGameMode`)))
        (if (`KismetArrayLibrary.Array_Contains` (`/Game/Blueprints/MainGameMode.MainTreeTiles` _asmain_game_mode) (`self.Tile`))
          (bind _returnvalue (`|CreateWidget` "/Game/Blueprints/LoseWidget.LoseWidget_C" (`GameplayStatics.GetPlayerController` 0)))
          (`UserWidget.AddToViewport` _returnvalue 0)
          (else
            (`|ExecutionSequence`
              (:`then_0`
                (cast `/Game/Blueprints/Buildings/Brambles` (`/Game/Blueprints/Tile.GroundBuilding` _tile))
                (if (`self.AffectsGround`)
                  (`self.K2_DestroyActor`)))
              (:`then_1`
                (cast `/Game/Blueprints/Buildings/UmbrellaLeaf` (`/Game/Blueprints/Tile.AirBuilding` _tile))
                (if (`self.AffectsAir`)
                  (`self.K2_DestroyActor`))))))))))

(fn `UserConstructionScript`)