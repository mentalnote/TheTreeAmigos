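; Orbit camera actor that serves as the player's view and rotates around a central pivot.
; On BeginPlay it pulls the Camera back along its forward vector by CameraDistance, registers itself with MainGameMode, then becomes player 0's view target.
; The Orbit function yaws the root by direction, OrbitSpeed and delta time, swinging the offset camera around the pivot; nothing in this Blueprint calls it.
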(event `self.ReceiveBeginPlay`
  (bind _camera (`self.Camera`))
  (`SceneComponent.K2_AddLocalOffset` _camera (* (`SceneComponent.GetForwardVector` _camera) (* (`self.CameraDistance`) -1.0)) false true)
  (bind _asmain_game_mode (cast `/Game/Blueprints/MainGameMode` (`GameplayStatics.GetGameMode`)))
  (set `/Game/Blueprints/MainGameMode.OrbitCamera` self _asmain_game_mode)
  (`PlayerController.SetViewTargetWithBlend` (`GameplayStatics.GetPlayerController` 0) self 0.0 "VTBlend_Linear" 0.0 false))

(event `self.ReceiveActorBeginOverlap`
  (params (OtherActor :type "Actor Object Reference")))

(fn `Orbit`
  (params (Direction :type "Float (double-precision)"))
  (`SceneComponent.K2_AddLocalRotation` (`self.DefaultSceneRoot`) (`KismetMathLibrary.MakeRotator` 0.0 0.0 (* (* Direction (`self.OrbitSpeed`)) (`GameplayStatics.GetWorldDeltaSeconds`))) false false))

(fn `UserConstructionScript`)