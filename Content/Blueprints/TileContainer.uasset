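; TileContainer spawns and stores a hexagonal grid of Tile actors, grown outward from the world origin.
; Initialize runs only while the tile list is empty, adding rings by filling each tile's missing neighbours at 60-degree steps and TileDistance spacing.
; Each new tile is linked both ways to its source and to adjacent existing tiles, using cyclic six-direction index math to avoid duplicate spawns.
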(event EventBeginPlay)

(event EventActorBeginOverlap
  (params (OtherActor :type Actor%20Object%20Reference)))

(event EventTick
  (params (DeltaSeconds :type Float%20%28single-precision%29)))

(fn ConstructionScript)

(fn Initialize
  (params (Radius :type Integer))
  (bind _tiles (Variables|Default|GetTiles))
  (if (== (Utilities|Array|Length (Variables|Default|GetTiles)) 0)
    (bind _returnvalue (Game|SpawnActorfromClass "/Game/Blueprints/Tile.Tile_C" (Math|Transform|MakeTransform "0, 0, 0") "AlwaysSpawn" 0 0))
    (Utilities|Array|Add (Variables|Default|GetTiles) _returnvalue)
    (for _index (range 0 Radius)
      (bind _output_get (LocalVariables|SetTilesLength (Utilities|Array|Length _tiles)))
      (for _index_2 (range 0 (- _output_get 1))
        (for _index_3 (range 0 5)
          (Utilities|IsValid (Utilities|Array|Get(acopy) (Variables|/Game/Blueprints/Tile.Tile_C|GetNeighbours (Utilities|Array|Get(acopy) _tiles _index_2)) _index_3)
            (:Is%20Not%20Valid
              (bind _returnvalue_2 (Game|SpawnActorfromClass "/Game/Blueprints/Tile.Tile_C" (Math|Transform|MakeTransform (+ (Transformation|GetActorLocation (Utilities|Array|Get(acopy) _tiles _index_2)) (Math|Vector|RotateVector (Math|Vector|MakeVector (Variables|Default|GetTileDistance) 0.0 0.0) (Math|Rotator|MakeRotator 0.0 0.0 (* (Math|Conversions|ToFloat(Integer) _index_3) 6e+01))))) "AlwaysSpawn" 0 0))
              (CallFunction|ConnectNeighbours _index_3 (Utilities|Array|Get(acopy) _tiles _index_2) _returnvalue_2)
              (Utilities|FlowControl|Sequence
                (:then_0
                  (bind _returnvalue_3 (CallFunction|CalculateCyclicIndex _index_3 1))
                  (Utilities|IsValid (Utilities|Array|Get(acopy) (Variables|/Game/Blueprints/Tile.Tile_C|GetNeighbours (Utilities|Array|Get(acopy) _tiles _index_2)) _returnvalue_3)
                    (:Is%20Valid
                      (bind _returnvalue_4 (CallFunction|CalculateCyclicIndex _returnvalue_3 -2))
                      (CallFunction|ConnectNeighbours _returnvalue_4 (Utilities|Array|Get(acopy) (Variables|/Game/Blueprints/Tile.Tile_C|GetNeighbours (Utilities|Array|Get(acopy) _tiles _index_2)) _returnvalue_3) _returnvalue_2))))
                (:then_1
                  (bind _returnvalue_5 (CallFunction|CalculateCyclicIndex _index_3 -1))
                  (Utilities|IsValid (Utilities|Array|Get(acopy) (Variables|/Game/Blueprints/Tile.Tile_C|GetNeighbours (Utilities|Array|Get(acopy) _tiles _index_2)) _returnvalue_5)
                    (:Is%20Valid
                      (bind _returnvalue_6 (CallFunction|CalculateCyclicIndex _returnvalue_5 2))
                      (CallFunction|ConnectNeighbours _returnvalue_6 (Utilities|Array|Get(acopy) (Variables|/Game/Blueprints/Tile.Tile_C|GetNeighbours (Utilities|Array|Get(acopy) _tiles _index_2)) _returnvalue_5) _returnvalue_2))))
                (:then_2
                  (Utilities|Array|Add (Variables|Default|GetTiles) _returnvalue_2))))))))))

(fn ConnectNeighbours
  (params (Neighbour :type Integer) (FromTile :type Tile%20Object%20Reference) (ToTile :type Tile%20Object%20Reference))
  (Utilities|Array|SetArrayElem (Variables|/Game/Blueprints/Tile.Tile_C|GetNeighbours FromTile) Neighbour ToTile)
  (Utilities|Array|SetArrayElem (Variables|/Game/Blueprints/Tile.Tile_C|GetNeighbours ToTile) (Utilities|Select :Index Neighbour :Option%200 3 :Option%201 4 :Option%202 5 :Option%203 0 :Option%204 1 :Option%205 2) FromTile))

(fn CalculateCyclicIndex
  (params (Index :type Integer) (Modification :type Integer))
  (LocalVariables|SetValue (Math|Integer|%(Integer) (+ Index Modification) 6))
  (if (< (LocalVariables|GetValue) 0) :!label _label
    (LocalVariables|SetValue (+ (LocalVariables|GetValue) 6))
    (goto _label)
    (else
      (return (LocalVariables|GetValue)))))