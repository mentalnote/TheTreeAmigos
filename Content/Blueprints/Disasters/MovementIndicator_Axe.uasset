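; Animated axe movement indicator actor, with three meshes arranged around its origin in a repeating chopping-style motion.
; Each tick sets the relative transform of all three, lerping between a raised and a lowered height while swinging the rotation.
; The shared alpha is a squared triangle wave with a one-second period, computed from real time so it ignores time dilation.
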(event `self.ReceiveBeginPlay`)

(event `self.ReceiveActorBeginOverlap`
  (params (OtherActor :type "Actor Object Reference")))

(event `self.ReceiveTick`
  (params (DeltaSeconds :type "Float (single-precision)"))
  (bind _returnvalue (`KismetMathLibrary.Square` (- 1.0 (`KismetMathLibrary.Abs` (* (- (mod (`GameplayStatics.GetRealTimeSeconds`) 1.0) 0.5) 2.0)))))
  (`SceneComponent.K2_SetRelativeTransform` (`self.Mesh1`) (`KismetMathLibrary.MakeTransform` (`KismetMathLibrary.VLerp` (50.0 0.0 40.0) (50.0 0.0 20.0) _returnvalue) (`KismetMathLibrary.RLerp` (struct :`Pitch` 50.0 :`Roll` 90.0) (struct :`Pitch` 70.0 :`Roll` 90.0) _returnvalue)) false true)
  (`SceneComponent.K2_SetRelativeTransform` (`self.Mesh2`) (`KismetMathLibrary.MakeTransform` (`KismetMathLibrary.VLerp` (-30.0 20.0 40.0) (-30.0 20.0 20.0) _returnvalue) (`KismetMathLibrary.RLerp` (struct :`Pitch` 50.0 :`Yaw` 140.0 :`Roll` 90.0) (struct :`Pitch` 70.0 :`Yaw` 140.0 :`Roll` 90.0) _returnvalue)) false false)
  (`SceneComponent.K2_SetRelativeTransform` (`self.Mesh3`) (`KismetMathLibrary.MakeTransform` (`KismetMathLibrary.VLerp` (-20.0 -40.0 40.0) (-20.0 -40.0 20.0) _returnvalue) (`KismetMathLibrary.RLerp` (struct :`Pitch` 50.0 :`Yaw` -120.0 :`Roll` 90.0) (struct :`Pitch` 70.0 :`Yaw` -120.0 :`Roll` 90.0) _returnvalue)) false false))

(fn `UserConstructionScript`)