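; Map tile actor that handles cursor hover and selection, holds ground and air buildings, and can spawn disasters.
; Hover and select meshes show state, with GameMode's MainTreeTiles highlighted as one group and SelectedTile tracking the selection.
; Construct spawns a ground building, while Salvage refunds sunlight and water and destroys the building only when collecting resources.
; AffectTile passes air or ground buildings to Salvage without collection, according to the disaster's flags.
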(event `self.ReceiveBeginPlay`)

(event `self.ReceiveActorBeginCursorOver`
  (bind _asmain_game_mode (cast `/Game/Blueprints/MainGameMode` (`GameplayStatics.GetGameMode`))
    (:`then`
      (bind _maintreetiles (`/Game/Blueprints/MainGameMode.MainTreeTiles` _asmain_game_mode))
      (if (`KismetArrayLibrary.Array_Contains` _maintreetiles self)
        (for _array_element _maintreetiles
          (`self.HoverOver` _array_element))
        (else
          (`self.HoverOver` :!label _label)
          (for _array_element_2 _maintreetiles
            (`self.ExitHoverOver` _array_element_2)))))
    (:`CastFailed`
      (goto _label))))

(event `self.ReceiveActorEndCursorOver`
  (bind _asmain_game_mode (cast `/Game/Blueprints/MainGameMode` (`GameplayStatics.GetGameMode`))
    (:`then`
      (if (not (`KismetArrayLibrary.Array_Contains` (`/Game/Blueprints/MainGameMode.MainTreeTiles` _asmain_game_mode) self))
        (`self.ExitHoverOver` :!label _label_2)))
    (:`CastFailed`
      (goto _label_2))))

(event `self.ReceiveActorOnClicked`
  (`self.Select`))

(event `HoverOver`
  (`SceneComponent.SetVisibility` (`self.HoverMesh`) true false))

(event `ExitHoverOver`
  (`SceneComponent.SetVisibility` (`self.HoverMesh`) false false))

(event `AffectTile`
  (params (Disaster :type "/Game/Blueprints/Disaster Object Reference"))
  (if (`/Game/Blueprints/Disaster.AffectsAir` Disaster)
    (`self.Salvage` false (`self.AirBuilding`)))
  (if (`/Game/Blueprints/Disaster.AffectsGround` Disaster)
    (`self.Salvage` false (`self.GroundBuilding`))))

(fn `Construct`
  (params (BuidlingType :type "/Game/Blueprints/Buildings/Building Class Reference"))
  (`self.Salvage` false)
  (bind _returnvalue (`|SpawnActorFromClass` BuidlingType (`self.GetTransform`) "AlwaysSpawn" "OverrideRootScale"))
  (set `self.GroundBuilding` _returnvalue))

(fn `Salvage`
  (params (CollectResources :type Boolean) (Building :type "/Game/Blueprints/Buildings/Building Object Reference"))
  (`/Engine/EditorBlueprintResources/StandardMacros.IsValid` Building
    (:`Is Valid`
      (if CollectResources
        (bind _asmain_game_mode (cast `/Game/Blueprints/MainGameMode` (`GameplayStatics.GetGameMode`))
          (:`then`
            (bind _currency (`/Game/Blueprints/MainGameMode.Currency` _asmain_game_mode))
            (`/Game/Blueprints/Currency.AddSunlight` _currency (`/Game/Blueprints/Buildings/Building.SunlightCost` Building))
            (`/Game/Blueprints/Currency.AddWater` _currency (`/Game/Blueprints/Buildings/Building.WaterCost` Building)))
          (:`CastFailed`
            _))
        (`self.K2_DestroyActor` Building)))))

(fn `Select`
  (`SceneComponent.SetVisibility` (`self.SelectMesh`) true false)
  (bind _asmain_game_mode (cast `/Game/Blueprints/MainGameMode` (`GameplayStatics.GetGameMode`)))
  (bind _selectedtile (`/Game/Blueprints/MainGameMode.SelectedTile` _asmain_game_mode))
  (`/Engine/EditorBlueprintResources/StandardMacros.IsValid` _selectedtile
    (:`Is Valid`
      (if (not (== _selectedtile self))
        (bind _maintreetiles (`/Game/Blueprints/MainGameMode.MainTreeTiles` _asmain_game_mode))
        (bind _returnvalue (`KismetArrayLibrary.Array_Contains` _maintreetiles self))
        (if (and (not _returnvalue) (`KismetArrayLibrary.Array_Contains` _maintreetiles _selectedtile))
          (for _array_element _maintreetiles
            (`SceneComponent.SetVisibility` (`/Game/Blueprints/Tile.SelectMesh` _array_element) false false))
          (else
            (`self.Unselect` _selectedtile)))))
    (:`Is Not Valid`
      _))
  (set `/Game/Blueprints/MainGameMode.SelectedTile` self _asmain_game_mode)
  (if _returnvalue
    (for _array_element_2 _maintreetiles
      (`SceneComponent.SetVisibility` (`/Game/Blueprints/Tile.SelectMesh` _array_element_2) true false))))

(fn `SpawnDisaster`
  (params (NewDisaster :type "/Game/Blueprints/Disaster Class Reference"))
  (`/Engine/EditorBlueprintResources/StandardMacros.IsValid` (`self.Disaster`)
    (:`Is Not Valid`
      (bind _returnvalue (`|SpawnActorFromClass` NewDisaster (`self.GetTransform`) "AlwaysSpawn" "OverrideRootScale"))
      (`/Game/Blueprints/Disaster.MoveToTile` _returnvalue self false))))

(fn `Unselect`
  (`SceneComponent.SetVisibility` (`self.SelectMesh`) false false))

(fn `UserConstructionScript`
  (set `self.Neighbours` (`|MakeArray` null null null null null null :!type "/Game/Blueprints/Tile Object Reference")))