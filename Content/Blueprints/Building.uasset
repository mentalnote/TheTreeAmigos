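; Building Blueprint that decides whether it can be constructed on a given tile.
; CanConstruct requires the tile's existing building to be exactly the RequiredBase class, or the tile to be empty when no base is required, so buildings can act as upgrades of others.
; It then checks SunlightCost and WaterCost against the Currency held by MainGameMode, without deducting either resource.
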(fn `CanConstruct`
  (params (Tile :type "/Game/Blueprints/Tile Object Reference"))
  (returns (CanConstruct :type Boolean))
  (bind _buidling (`/Game/Blueprints/Tile.Buidling` Tile))
  (`/Engine/EditorBlueprintResources/StandardMacros.IsValid` _buidling
    (:`Is Valid`
      (if (== (`GameplayStatics.GetObjectClass` _buidling) (`self.RequiredBase`))
        (bind _asmain_game_mode (cast `/Game/Blueprints/MainGameMode` (`GameplayStatics.GetGameMode`) :!label _label)
          (:`then`
            (bind _currency (`/Game/Blueprints/MainGameMode.Currency` _asmain_game_mode))
            (bind _sunlight (`/Game/Blueprints/Currency.GetSunlight` _currency))
            (if (<= (`self.SunlightCost`) _sunlight)
              (bind _water (`/Game/Blueprints/Currency.GetWater` _currency))
              (if (<= (`self.WaterCost`) _water)
                (return true)
                (else
                  _))))
          (:`CastFailed`
            _))))
    (:`Is Not Valid`
      (if (!= (`self.RequiredBase`) null)
        _
        (else
          (goto _label)))))
  (return false))

(fn `UserConstructionScript`)